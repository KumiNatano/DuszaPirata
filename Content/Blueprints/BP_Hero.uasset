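; BP_Hero is the player hero Blueprint, handling camera setup, health bar updates and the death screen.
; BeginPlay binds the death event, sets game-only input with a hidden cursor and locks camera pitch to a fixed downward angle.
; RefreshHPBar passes HealthSystem values to BP_HeroController, while death shows WB_DeathScreen and the cursor.
; An unconnected barrel-kick prototype using sphere overlap and impulse never runs.
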(event Custom|RefreshHPBar
  (bind _healthsystem (Variables|Default|GetHealthSystem))
  (bind _asbp_hero_controller (Utilities|Casting|CastToBP_HeroController (Pawn|GetController)))
  (Default|UpdateHealthBar _asbp_hero_controller (Variables|/Script/DuszaPirata.HealthSystem|GetHealth _healthsystem) (Variables|/Script/DuszaPirata.HealthSystem|GetMaxHealth _healthsystem)))

(event Custom|OnHeroDeathBP_Event
  (bind _returnvalue (UserInterface|CreateWidget "/Game/UI/WB_DeathScreen.WB_DeathScreen_C"))
  (UserInterface|Viewport|AddtoViewport _returnvalue 0)
  (Variables|/Script/Engine.PlayerController|SetbShowMouseCursor (Game|GetPlayerController 0) true))

(event EventBeginPlay
  (bind _returnvalue (Game|GetPlayerController 0))
  (bind _returnvalue_2 (Game|GetPlayerCameraManager 0))
  (EventDispatchers|AssignOnHeroDeathBP (delegate Custom|OnHeroDeathBP_Event))
  (Variables|/Script/Engine.PlayerController|SetbShowMouseCursor _returnvalue false)
  (Input|SetInputModeGameOnly _returnvalue false)
  (Utilities|Casting|CastToBP_HeroController (Pawn|GetController))
  (Variables|/Script/Engine.PlayerCameraManager|SetViewPitchMin _returnvalue_2 -6e+01)
  (Variables|/Script/Engine.PlayerCameraManager|SetViewPitchMax _returnvalue_2 -6e+01))

(fn ConstructionScript)